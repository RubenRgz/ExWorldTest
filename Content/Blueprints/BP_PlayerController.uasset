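; Player controller that toggles the audio settings menu on the HUD.
; The OpenAudioMenu input shows the menu widget held by BP_HUD, switches to Game and UI input and shows the mouse cursor.
; OnCloseAudioMenu hides the widget, restores game-only input and hides the cursor, with an IsAudioMenuOpen flag preventing repeated opens.
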(event `InputAction|OpenAudioMenu`
  (params (Key :type "Key Structure"))
  (:`Pressed`
    (if (not (`self.IsAudioMenuOpen`))
      (bind _asbp_hud (cast `/Game/Blueprints/BP_HUD` (`self.GetHUD`)))
      (`Widget.SetVisibility` (`/Game/Widgets/WB_HUD.WB_AudioMenu` (`/Game/Blueprints/BP_HUD.HUDWidgetRef` _asbp_hud)) "Visible")
      (`WidgetBlueprintLibrary.SetInputMode_GameAndUIEx` self null)
      (set `self.bShowMouseCursor` true)
      (set `self.IsAudioMenuOpen` true))))

(event `OnCloseAudioMenu`
  (bind _asbp_hud (cast `/Game/Blueprints/BP_HUD` (`self.GetHUD`)))
  (`Widget.SetVisibility` (`/Game/Widgets/WB_HUD.WB_AudioMenu` (`/Game/Blueprints/BP_HUD.HUDWidgetRef` _asbp_hud)) "Hidden")
  (`WidgetBlueprintLibrary.SetInputMode_GameOnly` self)
  (set `self.bShowMouseCursor` false)
  (set `self.IsAudioMenuOpen` false))

(fn `UserConstructionScript`)